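; Blueprint that receives OSC messages over the network and turns accelerometer input into an AccelX value.
; On BeginPlay it creates a listening OSC server on a hard-coded IP and port and binds a message handler.
; The handler matches the last address segment against Accel, reads the first float, stores it above a small deadzone or zero otherwise (including negatives), and prints the result.
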(event Custom|OSCIn
  (params (Message :type OSC%20Message%20Structure%20%28by%20ref%29) (IPAddress :type String) (Port :type Integer))
  (bind _output_get (Variables|Default|SetOSCMessages Message))
  (bind _returnvalue (Class|OSCManager|GetOSCMessageAddress _output_get))
  (bind _returnvalue_2 (Class|OSCManager|GetOSCAddressFullPath _returnvalue))
  (switch string (.RightS (Utilities|String|Split _returnvalue_2 "/" "IgnoreCase" "FromEnd"))
    (:accel
      (bind _value (Class|OSCManager|GetFloat (Variables|Default|GetOSCMessages)))
      (if (> _value 0.01)
        (bind _output_get_2 (Variables|Default|SetAccelX (Math|Float|Absolute(Float) _value)))
        (Development|PrintString (Utilities|String|ToString(Float) _output_get_2))
        (else
          (bind _output_get_3 (Variables|Default|SetAccelX 0.0))
          (Development|PrintString (Utilities|String|ToString(Float) _output_get_3)))))))

(event EventBeginPlay
  (bind _returnvalue (Class|OSCManager|CreateOSCServer "140.113.66.100" 7000 false true "" 0))
  (bind _output_get (Variables|Default|SetOSCServer _returnvalue))
  (EventDispatchers|BindEventtoOnOscMessageReceived _output_get (EventDispatchers|CreateEvent :!event Custom|OSCIn)))

(event EventTick
  (params (DeltaSeconds :type Float%20%28single-precision%29)))

(fn ConstructionScript)