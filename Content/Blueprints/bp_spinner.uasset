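; A physics-driven two-arm spinner actor that leaves a colored Niagara trail and is pushed by X acceleration read from BpOsc.
; Each tick, Arm1 receives an impulse at an arrow component, scaled by that input and a multiplier randomized per instance at BeginPlay.
; The construction script applies SpinnerColor to emissive dynamic materials on Arm2 and adjusts its bar scale and part offsets from Arm2Scale.
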(event Custom|ImpulseArm1
  (bind _impulsearrow (Variables|Default|GetImpulseArrow))
  (bind _returnvalue (Transformation|GetWorldLocation _impulsearrow))
  (Physics|AddImpulseatLocation (Variables|Default|GetArm1) (+ (* (Math|Vector|GetForwardVector _impulsearrow) (* (Variables|Default|GetAccel%20X) (Variables|Default|GetImpulseScalar))) _returnvalue) _returnvalue "None"))

(event EventBeginPlay
  (bind _returnvalue (Niagara|SpawnSystemAttached "/Game/NS/NS_Trail.NS_Trail" (Variables|Default|GetNiagaraPos) "None" "0, 0, 0" "0, 0, 0" "KeepRelativeOffset" false))
  (bind _output_get (Variables|Default|SetNS_Trail _returnvalue))
  (Effects|Components|ParticleSystem|SetColorParameter _output_get "User.Color" (Variables|Default|GetSpinnerColor))
  (Variables|Default|SetImpulseScalar (* (Variables|Default|GetImpulseScalar) (Math|Random|RandomFloatinRange 1.0 2.0))))

(event EventTick
  (params (DeltaSeconds :type Float%20%28single-precision%29))
  (Variables|Default|SetAccel%20X (Variables|/Game/Blueprints/bp_osc.bp_osc_C|GetAccelX (Variables|Default|Getbp_osc)))
  (CallFunction|ImpulseArm1))

(fn ConstructionScript
  (bind _arm2scale (Variables|Default|GetArm2Scale))
  (bind _returnvalue (- _arm2scale 1.0))
  (bind _returnvalue_2 (* _returnvalue 8e+01))
  (Utilities|FlowControl|Sequence
    (:then_0
      (bind _returnvalue_3 (Rendering|Material|CreateDynamicMaterialInstance (Variables|Default|GetArm2Bar) 0 "/Game/Materials/mt_emissive.mt_emissive" "None" :!class /Script/Engine.PrimitiveComponent))
      (bind _output_get (Variables|Default|SetM_Arm2Bar _returnvalue_3))
      (Rendering|Material|SetVectorParameterValue _output_get "Color" (Variables|Default|GetSpinnerColor) :!class /Script/Engine.MaterialInstanceDynamic)
      (bind _returnvalue_4 (Rendering|Material|CreateDynamicMaterialInstance (Variables|Default|GetArm2Light) 0 "/Game/Materials/mt_emissive.mt_emissive" "None" :!class /Script/Engine.PrimitiveComponent))
      (bind _output_get_2 (Variables|Default|SetM_Arm2Light _returnvalue_4))
      (Rendering|Material|SetVectorParameterValue _output_get_2 "Color" (Variables|Default|GetSpinnerColor) :!class /Script/Engine.MaterialInstanceDynamic))
    (:then_1
      (Transformation|SetRelativeScale3D (Variables|Default|GetArm2Bar) (Math|Vector|MakeVector 1.0 1.0 _arm2scale))
      (Transformation|AddLocalOffset (Variables|Default|GetArm2Bar) (Math|Vector|MakeVector 0.0 0.0 _returnvalue_2) false false)
      (Transformation|SetRelativeLocation (Variables|Default|GetArm2Start) (Variables|/Script/Engine.SceneComponent|GetRelativeLocation (Variables|Default|GetArm2Bar)) false false)
      (Transformation|AddLocalOffset (Variables|Default|GetArm2End) (Math|Vector|MakeVector 0.0 0.0 (* _returnvalue_2 -1.0)) false false))))